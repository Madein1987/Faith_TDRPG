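; BP_RandomEncounter is an actor that triggers a battle when the player character touches it.
; On BeginPlay it moves to a random X and Y position within a fixed range.
; Its capsule overlap casts to BP_MasterCharacter, stores the player's transform and a stored-position flag in the game instance reference, then opens the battle test map after a short delay.
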(event OnComponentBeginOverlap(Capsule)
  (params (OverlappedComponent :type Primitive%20Component%20Object%20Reference) (OtherActor :type Actor%20Object%20Reference) (OtherComp :type Primitive%20Component%20Object%20Reference) (OtherBodyIndex :type Integer) (bFromSweep :type Boolean) (SweepResult :type Hit%20Result%20Structure%20%28by%20ref%29))
  (bind _asbp_master_character (Utilities|Casting|CastToBP_MasterCharacter OtherActor))
  (bind _output_get (Variables|Default|Set_BP_Master_Character_Reference _asbp_master_character))
  (Variables|/Game/GI_Faith.GI_Faith_C|Set_GI_bHasStoredPosition? (Variables|/Game/CHARACTERS/BP_MasterCharacter.BP_MasterCharacter_C|Get_GI_Faith_Reference _output_get) true)
  (Variables|/Game/GI_Faith.GI_Faith_C|Set_GI_PlayerPosition (Variables|/Game/CHARACTERS/BP_MasterCharacter.BP_MasterCharacter_C|Get_GI_Faith_Reference _output_get) (Transformation|GetActorTransform _asbp_master_character))
  (Utilities|FlowControl|Delay 1.0)
  (Game|OpenLevel(byName) "Test_BattleMap"))

(event EventBeginPlay
  (bind _returnvalue (Math|Random|RandomFloatinRange 0.0 3e+03))
  (Transformation|SetActorLocation (Math|Vector|MakeVector _returnvalue _returnvalue 0.0) false false))

(event Collision|EventActorBeginOverlap
  (params (OtherActor :type Actor%20Object%20Reference)))

(event EventTick
  (params (DeltaSeconds :type Float%20%28single-precision%29)))

(fn ConstructionScript)