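; Combat-mode player character that drives a slide-in combat menu with Enhanced Input.
; BeginPlay adds the combat mapping context and, only if the game instance holds a stored position, moves the character there and shows the menu.
; D-pad up/down cycles the menu selection with wraparound and debug prints, while Teleport opens the test overworld map.
; Left/right and Interact are empty; movement, jump-animation and menu-toggle logic is left unwired.
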(event EventBeginPlay
  (bind __gi_faith_reference (Variables|Default|Get_GI_Faith_Reference))
  (|CallParentFunction)
  (bind _asplayer_controller (Utilities|Casting|CastToPlayerController (Pawn|GetController)))
  (Input|AddMappingContext (PlayerController|LocalPlayerSubsystems|GetEnhancedInputLocalPlayerSubsystem _asplayer_controller) "/Game/INPUTS/IMC_Faith_00_Combat.IMC_Faith_00_Combat" 0 "(bIgnoreAllPressedKeysUntilRelease=True,bForceImmediately=False,bNotifyUserSettings=False)")
  (if (Variables|/Game/GI_Faith.GI_Faith_C|Get_GI_bHasStoredPosition? __gi_faith_reference)
    (Transformation|SetActorTransform (Variables|/Game/GI_Faith.GI_Faith_C|Get_GI_PlayerPosition __gi_faith_reference))
    (bind _returnvalue (UserInterface|CreateWidget "/Game/GUI/WBP_CombatMenu.WBP_CombatMenu_C" (Game|GetPlayerController 0)))
    (Variables|Default|Set_CombatMenuReference _returnvalue)
    (UserInterface|Viewport|AddtoPlayerScreen _returnvalue)
    (UserInterface|Animation|PlayAnimation _returnvalue (Variables|/Game/GUI/WBP_CombatMenu.WBP_CombatMenu_C|GetSlideIn _returnvalue) 0.0 1 "Forward" 1.0 false)))

(event Collision|EventActorBeginOverlap
  (params (OtherActor :type Actor%20Object%20Reference))
  (|CallParentFunction OtherActor) ; This node is disabled and will not be called.\nDrag off pins to build functionality.
)

(event EventTick
  (params (DeltaSeconds :type Float%20%28single-precision%29))
  (|CallParentFunction DeltaSeconds))

(event Input|EnhancedActionEvents|EnhancedInputActionIA_DPad_MoveLeft
  (params (ActionValue :type Float%20%28double-precision%29) (ElapsedSeconds :type Float%20%28double-precision%29) (TriggeredSeconds :type Float%20%28double-precision%29) (InputAction :type Input%20Action%20Object%20Reference :default "/Game/INPUTS/IA_DPad_MoveLeft.IA_DPad_MoveLeft")))

(event Input|EnhancedActionEvents|EnhancedInputActionIA_DPad_MoveRight
  (params (ActionValue :type Float%20%28double-precision%29) (ElapsedSeconds :type Float%20%28double-precision%29) (TriggeredSeconds :type Float%20%28double-precision%29) (InputAction :type Input%20Action%20Object%20Reference :default "/Game/INPUTS/IA_DPad_MoveRight.IA_DPad_MoveRight")))

(event Input|EnhancedActionEvents|EnhancedInputActionIA_Teleport
  (params (ActionValue :type Boolean) (ElapsedSeconds :type Float%20%28double-precision%29) (TriggeredSeconds :type Float%20%28double-precision%29) (InputAction :type Input%20Action%20Object%20Reference :default "/Game/INPUTS/IA_Teleport.IA_Teleport"))
  (:Started
    (Game|OpenLevel(byName) "Test_OverworldMap")))

(event Input|EnhancedActionEvents|EnhancedInputActionIA_ToogleCombatMenu
  (params (ActionValue :type Boolean) (ElapsedSeconds :type Float%20%28double-precision%29) (TriggeredSeconds :type Float%20%28double-precision%29) (InputAction :type Input%20Action%20Object%20Reference :default "/Game/INPUTS/IA_ToogleCombatMenu.IA_ToogleCombatMenu")))

(event Input|EnhancedActionEvents|EnhancedInputActionIA_Interact
  (params (ActionValue :type Boolean) (ElapsedSeconds :type Float%20%28double-precision%29) (TriggeredSeconds :type Float%20%28double-precision%29) (InputAction :type Input%20Action%20Object%20Reference :default "/Game/INPUTS/IA_Interact.IA_Interact")))

(event Input|EnhancedActionEvents|EnhancedInputActionIA_DPad_NavigateDown
  (params (ActionValue :type Boolean) (ElapsedSeconds :type Float%20%28double-precision%29) (TriggeredSeconds :type Float%20%28double-precision%29) (InputAction :type Input%20Action%20Object%20Reference :default "/Game/INPUTS/IA_DPad_NavigateDown.IA_DPad_NavigateDown"))
  (bind __combatmenureference (Variables|Default|Get_CombatMenuReference))
  (:Started
    (bind _result (Math|Integer|IncrementInt (Variables|/Game/GUI/WBP_CombatMenu.WBP_CombatMenu_C|Getvar_CurrentMenuSelectionID __combatmenureference))
      (:%20%20
        (if (> _result (- (Variables|/Game/GUI/WBP_CombatMenu.WBP_CombatMenu_C|Getvar_NbreOfEntry __combatmenureference) 1))
          (Variables|/Game/GUI/WBP_CombatMenu.WBP_CombatMenu_C|Setvar_CurrentMenuSelectionID __combatmenureference 0))
        (Development|PrintString (Utilities|String|ToString(Integer) (Variables|/Game/GUI/WBP_CombatMenu.WBP_CombatMenu_C|Getvar_CurrentMenuSelectionID __combatmenureference)) true true "(R=0.085560,G=1.000000,B=0.157687,A=1.000000)")))))

(event Input|EnhancedActionEvents|EnhancedInputActionIA_DPad_NavigateUp
  (params (ActionValue :type Boolean) (ElapsedSeconds :type Float%20%28double-precision%29) (TriggeredSeconds :type Float%20%28double-precision%29) (InputAction :type Input%20Action%20Object%20Reference :default "/Game/INPUTS/IA_DPad_NavigateUp.IA_DPad_NavigateUp"))
  (bind __combatmenureference (Variables|Default|Get_CombatMenuReference))
  (:Started
    (bind _result (Math|Integer|DecrementInt (Variables|/Game/GUI/WBP_CombatMenu.WBP_CombatMenu_C|Getvar_CurrentMenuSelectionID __combatmenureference))
      (:%20%20
        (if (< _result 0)
          (Variables|/Game/GUI/WBP_CombatMenu.WBP_CombatMenu_C|Setvar_CurrentMenuSelectionID __combatmenureference (- (Variables|/Game/GUI/WBP_CombatMenu.WBP_CombatMenu_C|Getvar_NbreOfEntry __combatmenureference) 1)))
        (Development|PrintString (Utilities|String|ToString(Integer) (Variables|/Game/GUI/WBP_CombatMenu.WBP_CombatMenu_C|Getvar_CurrentMenuSelectionID __combatmenureference)) true true "(R=0.085560,G=1.000000,B=0.157687,A=1.000000)")))))

(fn ConstructionScript
  (|CallParentFunction))

(fn CombatMenuVisibility
  (if (Variables|Default|Getb_isCombatMenuVisible?)
    (Utilities|IsValid (Variables|Default|Get_CombatMenuReference)
      (:Is%20Not%20Valid
        (bind _returnvalue (UserInterface|CreateWidget "/Game/GUI/WBP_CombatMenu.WBP_CombatMenu_C"))
        (bind _output_get (Variables|Default|Set_CombatMenuReference _returnvalue))
        (UserInterface|Viewport|AddtoPlayerScreen _output_get)))
    (else
      (UserInterface|Animation|PlayAnimation (Variables|Default|Get_CombatMenuReference) (Variables|/Game/GUI/WBP_CombatMenu.WBP_CombatMenu_C|GetSlideInOut (Variables|Default|Get_CombatMenuReference)) 0.0 1 "Reverse" 1.0 false))))