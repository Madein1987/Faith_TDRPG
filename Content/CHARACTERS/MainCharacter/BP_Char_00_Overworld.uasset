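; Overworld player character with four-direction D-pad movement and directional sprite animation.
; On BeginPlay it adds the Faith input mapping context and restores any transform stored in the GameInstance reference.
; Axis flags block diagonal movement, and a DoOnce per direction fires one animation JumpToNode per press, resetting on release or cancel.
; The Teleport input opens the test overworld map.
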(event EventBeginPlay
  (bind __gi_faith_reference (Variables|Default|Get_GI_Faith_Reference))
  (|CallParentFunction)
  (bind _asplayer_controller (Utilities|Casting|CastToPlayerController (Pawn|GetController)))
  (Input|AddMappingContext (PlayerController|LocalPlayerSubsystems|GetEnhancedInputLocalPlayerSubsystem _asplayer_controller) "/Game/INPUTS/IMC_Faith_00.IMC_Faith_00" 0 "(bIgnoreAllPressedKeysUntilRelease=True,bForceImmediately=False,bNotifyUserSettings=False)")
  (if (Variables|/Game/GI_Faith.GI_Faith_C|Get_GI_bHasStoredPosition? __gi_faith_reference)
    (Transformation|SetActorTransform (Variables|/Game/GI_Faith.GI_Faith_C|Get_GI_PlayerPosition __gi_faith_reference))))

(event Collision|EventActorBeginOverlap
  (params (OtherActor :type Actor%20Object%20Reference))
  (|CallParentFunction OtherActor) ; This node is disabled and will not be called.\nDrag off pins to build functionality.
)

(event EventTick
  (params (DeltaSeconds :type Float%20%28single-precision%29))
  (|CallParentFunction DeltaSeconds) ; This node is disabled and will not be called.\nDrag off pins to build functionality.
)

(event Input|EnhancedActionEvents|EnhancedInputActionIA_DPad_MoveDown
  (params (ActionValue :type Float%20%28double-precision%29) (ElapsedSeconds :type Float%20%28double-precision%29) (TriggeredSeconds :type Float%20%28double-precision%29) (InputAction :type Input%20Action%20Object%20Reference :default "/Game/INPUTS/IA_DPad_MoveDown.IA_DPad_MoveDown"))
  (:Triggered
    (if (not (Variables|Default|Getb_IsMoving_X?))
      (Variables|Default|Setb_IsMoving_Y? true)
      (Pawn|Input|AddMovementInput (Math|Vector|MakeVector 0.0 1.0 0.0) 1.0 false)
      (Utilities|FlowControl|DoOnce false :!label _label
        (:Completed
          (Class|PaperZDAnimInstance|JumptoNode (Variables|/Script/PaperZD.PaperZDAnimationComponent|GetAnimInstance (Variables|Default|GetAnimationComponent)) "JumpDown" "None")))))
  (:Canceled
    (Variables|Default|Setb_IsMoving_Y? false :!label _label_2)
    (goto _label Reset))
  (:Completed
    (goto _label_2)))

(event Input|EnhancedActionEvents|EnhancedInputActionIA_DPad_MoveUp
  (params (ActionValue :type Float%20%28double-precision%29) (ElapsedSeconds :type Float%20%28double-precision%29) (TriggeredSeconds :type Float%20%28double-precision%29) (InputAction :type Input%20Action%20Object%20Reference :default "/Game/INPUTS/IA_DPad_MoveUp.IA_DPad_MoveUp"))
  (:Triggered
    (if (not (Variables|Default|Getb_IsMoving_X?))
      (Variables|Default|Setb_IsMoving_Y? true)
      (Pawn|Input|AddMovementInput (Math|Vector|MakeVector 0.0 -1.0 0.0) 1.0 false)
      (Utilities|FlowControl|DoOnce false :!label _label
        (:Completed
          (Class|PaperZDAnimInstance|JumptoNode (Variables|/Script/PaperZD.PaperZDAnimationComponent|GetAnimInstance (Variables|Default|GetAnimationComponent)) "JumpUp" "None")))))
  (:Canceled
    (Variables|Default|Setb_IsMoving_Y? false :!label _label_2)
    (goto _label Reset))
  (:Completed
    (goto _label_2)))

(event Input|EnhancedActionEvents|EnhancedInputActionIA_DPad_MoveLeft
  (params (ActionValue :type Float%20%28double-precision%29) (ElapsedSeconds :type Float%20%28double-precision%29) (TriggeredSeconds :type Float%20%28double-precision%29) (InputAction :type Input%20Action%20Object%20Reference :default "/Game/INPUTS/IA_DPad_MoveLeft.IA_DPad_MoveLeft"))
  (:Triggered
    (if (not (Variables|Default|Getb_IsMoving_Y?))
      (Variables|Default|Setb_IsMoving_X? true)
      (Pawn|Input|AddMovementInput (Math|Vector|MakeVector -1.0 0.0 0.0) 1.0 false)
      (Utilities|FlowControl|DoOnce false :!label _label
        (:Completed
          (Class|PaperZDAnimInstance|JumptoNode (Variables|/Script/PaperZD.PaperZDAnimationComponent|GetAnimInstance (Variables|Default|GetAnimationComponent)) "JumpLeft" "None")))))
  (:Canceled
    (Variables|Default|Setb_IsMoving_X? false :!label _label_2)
    (goto _label Reset))
  (:Completed
    (goto _label_2)))

(event Input|EnhancedActionEvents|EnhancedInputActionIA_DPad_MoveRight
  (params (ActionValue :type Float%20%28double-precision%29) (ElapsedSeconds :type Float%20%28double-precision%29) (TriggeredSeconds :type Float%20%28double-precision%29) (InputAction :type Input%20Action%20Object%20Reference :default "/Game/INPUTS/IA_DPad_MoveRight.IA_DPad_MoveRight"))
  (:Triggered
    (if (not (Variables|Default|Getb_IsMoving_Y?))
      (Variables|Default|Setb_IsMoving_X? true)
      (Pawn|Input|AddMovementInput (Math|Vector|MakeVector 1.0 0.0 0.0) 1.0 false)
      (Utilities|FlowControl|DoOnce false :!label _label
        (:Completed
          (Class|PaperZDAnimInstance|JumptoNode (Variables|/Script/PaperZD.PaperZDAnimationComponent|GetAnimInstance (Variables|Default|GetAnimationComponent)) "JumpRight" "None")))))
  (:Canceled
    (Variables|Default|Setb_IsMoving_X? false :!label _label_2)
    (goto _label Reset))
  (:Completed
    (goto _label_2)))

(event Input|EnhancedActionEvents|EnhancedInputActionIA_Teleport
  (params (ActionValue :type Boolean) (ElapsedSeconds :type Float%20%28double-precision%29) (TriggeredSeconds :type Float%20%28double-precision%29) (InputAction :type Input%20Action%20Object%20Reference :default "/Game/INPUTS/IA_Teleport.IA_Teleport"))
  (:Started
    (Game|OpenLevel(byName) "Test_OverworldMap")))

(fn ConstructionScript
  (|CallParentFunction))